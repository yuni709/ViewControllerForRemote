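; BP_ViewportController is an actor that puts cursor and circle UI widgets on screen when play begins.
; If the IsShowUI flag is set, BeginPlay creates one widget from each configurable class for the first player controller and adds it to the viewport.
; Both widget instances are stored in variables, and the Blueprint has no other logic.
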(event `self.ReceiveBeginPlay`
  (if (`self.isShowUI`)
    (`|ExecutionSequence`
      (:`then_0`
        (bind _returnvalue (`|CreateWidget` (`self.CursorUIClass`) (`GameplayStatics.GetPlayerController` 0)))
        (bind _output_get (set `self.CursorUIInstance` _returnvalue))
        (`UserWidget.AddToViewport` _output_get 0))
      (:`then_1`
        (bind _returnvalue_2 (`|CreateWidget` (`self.CircleUIClass`) (`GameplayStatics.GetPlayerController` 0)))
        (bind _output_get_2 (set `self.CircleUIInstance` _returnvalue_2))
        (`UserWidget.AddToViewport` _output_get_2 0)))))

(fn `UserConstructionScript`)